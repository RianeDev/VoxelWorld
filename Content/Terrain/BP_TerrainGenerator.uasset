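; Terrain generator actor that spawns a BiomeX by BiomeY grid of BP_Chunk actors on BeginPlay.
; CreateBiomes runs nested countdown loops, offsetting each chunk along X by Spacing from the previous chunk's ProceduralMesh transform, with debug prints.
; The Y row step sits inside the X loop behind an XCount <= 0 check that never passes, so YCount never decrements.
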(event EventBeginPlay
  (CallFunction|CreateBiomes))

(fn ConstructionScript)

(fn CreateBiomes
  ;[1 1 1] Start Y loop
  (Variables|Default|SetYCount (Variables|Default|GetBiomeY))
  (while (> (Variables|Default|GetYCount) 0)
    (Development|PrintString (Utilities|String|Append "Y: " (Utilities|String|ToString(Integer) (Variables|Default|GetYCount))) true true "(R=0.000000,G=1.000000,B=0.000000,A=1.000000)" 2e+01)
    ;[1 1 1] Start X loop
    (Variables|Default|SetXCount (Variables|Default|GetBiomeX))
    (while (> (Variables|Default|GetXCount) 0)
      ;[1 1 1] Check if first iteration and set location to 0 if so
      (if (and (== (Variables|Default|GetXCount) (Variables|Default|GetBiomeX)) (== (Variables|Default|GetYCount) (Variables|Default|GetBiomeY)))
        (Development|PrintString "Spawning chunk")
        (bind _returnvalue (Game|SpawnActorfromClass "/Game/Terrain/BP_Chunk.BP_Chunk_C" (Variables|Default|GetLastSpawnLocation) "AdjustIfPossibleButAlwaysSpawn" self 0.05 0.05 0))
        (bind _output_get (Variables|Default|SetChunkRef _returnvalue))
        (if (Utilities|IsValid _output_get)
          (Variables|Default|SetLastSpawnLocation (Transformation|GetWorldTransform (Variables|/Game/Terrain/BP_Chunk.BP_Chunk_C|GetProceduralMesh _output_get)))
          (Variables|Default|SetXCount (- (Variables|Default|GetXCount) 1)))
        (else
          ;[1 1 1] If not the first iteration, just create another chunk along the X row
          (bind _returnvalue_2 (Game|SpawnActorfromClass "/Game/Terrain/BP_Chunk.BP_Chunk_C" (Math|Transform|MakeTransform (Math|Vector|MakeVector (+ (.x (.location (Variables|Default|GetLastSpawnLocation))) (Variables|Default|GetSpacing)) (.y (.location (Variables|Default|GetLastSpawnLocation))) (.z (.location (Variables|Default|GetLastSpawnLocation)))) (.rotation (Variables|Default|GetLastSpawnLocation)) (.scale (Variables|Default|GetLastSpawnLocation))) "AdjustIfPossibleButAlwaysSpawn" self 0.05 0.05 0))
          (if (Utilities|IsValid _returnvalue_2)
            (Variables|Default|SetLastSpawnLocation (Transformation|GetWorldTransform (Variables|/Game/Terrain/BP_Chunk.BP_Chunk_C|GetProceduralMesh _returnvalue_2)))
            ;[1 1 1] Check if X has reached 0 yet. If not, continue cycling through X.
            (if (<= (Variables|Default|GetXCount) 0)
              ;[1 1 1] If X has reached end of its row, check if Y is 0 (no other columns)
              (if (> (Variables|Default|GetYCount) 0)
                ;[1 1 1] If Y has columns left, reset X back to 0, and move forward along Y axis to start another row.
                (Variables|Default|SetLastSpawnLocation (Math|Transform|MakeTransform (Math|Vector|MakeVector 0.0 (+ (.y (.location (Variables|Default|GetLastSpawnLocation))) (Variables|Default|GetSpacing)) (.z (.location (Variables|Default|GetLastSpawnLocation)))) (.rotation (Variables|Default|GetLastSpawnLocation)) (.scale (Variables|Default|GetLastSpawnLocation))))
                (Variables|Default|SetYCount (- (Variables|Default|GetYCount) 1))
                (Development|PrintString "Moving by Y" true true "(R=1.000000,G=0.000000,B=0.970384,A=1.000000)" 2e+01))
              (else
                (Variables|Default|SetXCount (- (Variables|Default|GetXCount) 1)))))))))
  (Development|PrintString "Finished spawning biomes." true true "(R=0.000000,G=0.660000,B=1.000000,A=1.000000)" 8.0))