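; Voxel terrain generator actor that builds a block landscape and lets the player place and remove blocks.
; The construction script fills a grid with Grass, Dirt and Stone instances, offsetting columns by three summed sine-product waves and picking material by height thresholds, with grass only on top.
; Left click traces from the follow camera and adds the toolbar-selected grass or dirt on the grid, without an inventory check.
; Right click removes the hit instance.
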(event EventBeginPlay
  (Input|EnableInput (Game|GetPlayerController 0)))

(event Input|MouseEvents|LeftMouseButton
  (params (Key :type Key%20Structure :default "None"))
  (bind _tilesize (Variables|Default|GetTileSize))
  (bind _returnvalue (Math|Conversions|ToFloat(Integer) _tilesize))
  (:Pressed
    (bind _asthird_person_character (Utilities|Casting|CastToThirdPersonCharacter (Game|GetPlayerCharacter 0)))
    (bind _outhit (Collision|LineTraceByChannel (Transformation|GetWorldLocation (Variables|/Game/ThirdPersonBP/Blueprints/ThirdPersonCharacter.ThirdPersonCharacter_C|GetFollowCamera _asthird_person_character)) (+ (Transformation|GetWorldLocation (Variables|/Game/ThirdPersonBP/Blueprints/ThirdPersonCharacter.ThirdPersonCharacter_C|GetFollowCamera _asthird_person_character)) (* (Math|Vector|GetForwardVector (Variables|/Game/ThirdPersonBP/Blueprints/ThirdPersonCharacter.ThirdPersonCharacter_C|GetFollowCamera _asthird_person_character)) 1e+03)) "TraceTypeQuery1" false 0 "None" false))
    (bind _asthird_person_character_2 (Utilities|Casting|CastToThirdPersonCharacter (Game|GetPlayerCharacter 0)))
    (Utilities|IsValid (Utilities|Select :Index (Variables|/Game/ThirdPersonBP/Blueprints/ThirdPersonCharacter.ThirdPersonCharacter_C|GetToolbarSelectInt _asthird_person_character_2) :Option%200 (Variables|Default|GetGrass) :Option%201 (Variables|Default|GetDirt))
      (:Is%20Valid
        (Components|InstancedStaticMesh|AddInstance (Utilities|Select :Index (Variables|/Game/ThirdPersonBP/Blueprints/ThirdPersonCharacter.ThirdPersonCharacter_C|GetToolbarSelectInt _asthird_person_character_2) :Option%200 (Variables|Default|GetGrass) :Option%201 (Variables|Default|GetDirt)) (Math|Transform|MakeTransform (Math|Vector|MakeVector (Math|Float|SnapToGrid(Float) (.X (Math|Vector|BreakVector (.ImpactPoint (Collision|BreakHitResult _outhit)))) _returnvalue) (Math|Float|SnapToGrid(Float) (.Y (Math|Vector|BreakVector (.ImpactPoint (Collision|BreakHitResult _outhit)))) _returnvalue) (Math|Float|SnapToGrid(Float) (.Z (Math|Vector|BreakVector (.ImpactPoint (Collision|BreakHitResult _outhit)))) _returnvalue))))))))

(event Input|MouseEvents|RightMouseButton
  (params (Key :type Key%20Structure :default "None"))
  (:Pressed
    (bind _asthird_person_character (Utilities|Casting|CastToThirdPersonCharacter (Game|GetPlayerCharacter 0)))
    (bind (_outhit _returnvalue) (Collision|LineTraceByChannel (Transformation|GetWorldLocation (Variables|/Game/ThirdPersonBP/Blueprints/ThirdPersonCharacter.ThirdPersonCharacter_C|GetFollowCamera _asthird_person_character)) (+ (Transformation|GetWorldLocation (Variables|/Game/ThirdPersonBP/Blueprints/ThirdPersonCharacter.ThirdPersonCharacter_C|GetFollowCamera _asthird_person_character)) (* (Math|Vector|GetForwardVector (Variables|/Game/ThirdPersonBP/Blueprints/ThirdPersonCharacter.ThirdPersonCharacter_C|GetFollowCamera _asthird_person_character)) 1e+03)) "TraceTypeQuery1" false 0 "None" false))
    (if _returnvalue
      (if (== (.HitComponent (Collision|BreakHitResult _outhit)) (Variables|Default|GetGrass))
        (Class|InstancedStaticMeshComponent|RemoveInstance (Variables|Default|GetGrass) (.HitItem (Collision|BreakHitResult _outhit)))
        (elif (== (.HitComponent (Collision|BreakHitResult _outhit)) (Variables|Default|GetDirt))
          (Class|InstancedStaticMeshComponent|RemoveInstance (Variables|Default|GetDirt) (.HitItem (Collision|BreakHitResult _outhit)))
          (elif (== (.HitComponent (Collision|BreakHitResult _outhit)) (Variables|Default|GetStone))
            (Class|InstancedStaticMeshComponent|RemoveInstance (Variables|Default|GetStone) (.HitItem (Collision|BreakHitResult _outhit)))))))))

(fn ConstructionScript
  (bind _frequency2 (Variables|Default|GetFrequency2))
  (bind _frequency3 (Variables|Default|GetFrequency3))
  (bind _tilesize (Variables|Default|GetTileSize))
  (bind _frequency1 (Variables|Default|GetFrequency1))
  (for _index (range 5 (- (Variables|Default|GetLength) 5))
    (for _index_2 (range 5 (- (Variables|Default|GetWidth) 5))
      (for _index_3 (range 0 (Variables|Default|GetHeight))
        (if (== _index_3 (Variables|Default|GetHeight)) ; Check if top layer
          (if (< (Math|Conversions|ToFloat(Integer) (+ (* _index_3 _tilesize) (* (Math|Float|Round (+ (* (Math|Trig|Sin(Degrees) (* _index _frequency1)) (Math|Trig|Sin(Degrees) (* _index_2 _frequency1)) (Variables|Default|GetHeight1)) (* (Math|Trig|Sin(Degrees) (* (* _index _frequency2) 0.7)) (Math|Trig|Sin(Degrees) (* _index_2 _frequency2)) (Variables|Default|GetHeight2)) (* (Math|Trig|Sin(Degrees) (* _index _frequency3)) (Math|Trig|Sin(Degrees) (* (* _index_2 _frequency3) 0.4)) (Variables|Default|GetHeight3)))) (Variables|Default|GetTileSize)))) (Math|Conversions|ToFloat(Integer) (* (+ (Variables|Default|GetDirtFloor) (Variables|Default|GetHeight)) (Variables|Default|GetTileSize))))
            (if (< (Math|Conversions|ToFloat(Integer) (+ (* _index_3 _tilesize) (* (Math|Float|Round (+ (* (Math|Trig|Sin(Degrees) (* _index _frequency1)) (Math|Trig|Sin(Degrees) (* _index_2 _frequency1)) (Variables|Default|GetHeight1)) (* (Math|Trig|Sin(Degrees) (* (* _index _frequency2) 0.7)) (Math|Trig|Sin(Degrees) (* _index_2 _frequency2)) (Variables|Default|GetHeight2)) (* (Math|Trig|Sin(Degrees) (* _index _frequency3)) (Math|Trig|Sin(Degrees) (* (* _index_2 _frequency3) 0.4)) (Variables|Default|GetHeight3)))) (Variables|Default|GetTileSize)))) (Math|Conversions|ToFloat(Integer) (* (+ (Variables|Default|GetStoneFloor) (Variables|Default|GetHeight)) (Variables|Default|GetTileSize)))) :!label _label
              (Components|InstancedStaticMesh|AddInstance (Variables|Default|GetStone) (Math|Conversions|ToTransform(Vector) (Math|Vector|MakeVector (Math|Conversions|ToFloat(Integer) (* _index _tilesize)) (Math|Conversions|ToFloat(Integer) (* _index_2 _tilesize)) (Math|Conversions|ToFloat(Integer) (+ (* _index_3 _tilesize) (* (Math|Float|Round (+ (* (Math|Trig|Sin(Degrees) (* _index _frequency1)) (Math|Trig|Sin(Degrees) (* _index_2 _frequency1)) (Variables|Default|GetHeight1)) (* (Math|Trig|Sin(Degrees) (* (* _index _frequency2) 0.7)) (Math|Trig|Sin(Degrees) (* _index_2 _frequency2)) (Variables|Default|GetHeight2)) (* (Math|Trig|Sin(Degrees) (* _index _frequency3)) (Math|Trig|Sin(Degrees) (* (* _index_2 _frequency3) 0.4)) (Variables|Default|GetHeight3)))) (Variables|Default|GetTileSize)))))))
              (else
                (Components|InstancedStaticMesh|AddInstance (Variables|Default|GetDirt) (Math|Conversions|ToTransform(Vector) (Math|Vector|MakeVector (Math|Conversions|ToFloat(Integer) (* _index _tilesize)) (Math|Conversions|ToFloat(Integer) (* _index_2 _tilesize)) (Math|Conversions|ToFloat(Integer) (+ (* _index_3 _tilesize) (* (Math|Float|Round (+ (* (Math|Trig|Sin(Degrees) (* _index _frequency1)) (Math|Trig|Sin(Degrees) (* _index_2 _frequency1)) (Variables|Default|GetHeight1)) (* (Math|Trig|Sin(Degrees) (* (* _index _frequency2) 0.7)) (Math|Trig|Sin(Degrees) (* _index_2 _frequency2)) (Variables|Default|GetHeight2)) (* (Math|Trig|Sin(Degrees) (* _index _frequency3)) (Math|Trig|Sin(Degrees) (* (* _index_2 _frequency3) 0.4)) (Variables|Default|GetHeight3)))) (Variables|Default|GetTileSize)))))))))
            (else
              (Components|InstancedStaticMesh|AddInstance (Variables|Default|GetGrass) (Math|Conversions|ToTransform(Vector) (Math|Vector|MakeVector (Math|Conversions|ToFloat(Integer) (* _index _tilesize)) (Math|Conversions|ToFloat(Integer) (* _index_2 _tilesize)) (Math|Conversions|ToFloat(Integer) (+ (* _index_3 _tilesize) (* (Math|Float|Round (+ (* (Math|Trig|Sin(Degrees) (* _index _frequency1)) (Math|Trig|Sin(Degrees) (* _index_2 _frequency1)) (Variables|Default|GetHeight1)) (* (Math|Trig|Sin(Degrees) (* (* _index _frequency2) 0.7)) (Math|Trig|Sin(Degrees) (* _index_2 _frequency2)) (Variables|Default|GetHeight2)) (* (Math|Trig|Sin(Degrees) (* _index _frequency3)) (Math|Trig|Sin(Degrees) (* (* _index_2 _frequency3) 0.4)) (Variables|Default|GetHeight3)))) (Variables|Default|GetTileSize)))))))))
          (else
            (goto _label)))))))