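; Chunk actor that builds one square tile of blocky, voxel-style heightmap terrain in its construction script.
; It creates a FastNoiseWrapper from its noise type and frequency, then samples 2D noise across a ChunkSize grid offset by the actor's world position, so neighboring chunks can line up.
; Each column adds one HCube instance at a height floored to whole cube steps, forming only the surface layer.
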(event EventBeginPlay)

(event Collision|EventActorBeginOverlap
  (params (OtherActor :type Actor%20Object%20Reference)))

(event EventTick
  (params (DeltaSeconds :type Float%20%28single-precision%29)))

(fn ConstructionScript
  (bind _returnvalue (Transformation|GetActorLocation))
  (bind _chunksize (Variables|Default|GetChunkSize))
  (bind _returnvalue_2 (- _chunksize 1))
  (bind _returnvalue_3 (/ _returnvalue 1e+02))
  (bind (_x _y) (Math|Vector|BreakVector _returnvalue_3))
  (bind _returnvalue_4 (Game|ConstructObjectfromClass "/Script/FastNoiseGenerator.FastNoiseWrapper" self))
  (Class|FastNoiseWrapper|SetupFastNoise _returnvalue_4 (Variables|Default|GetNoise%20Type) 1337 (Variables|Default|GetFrequency) "Quintic" "FBM" 3 2.0 0.5 0.45 "Euclidean" "CellValue")
  (for _index (range 0 _returnvalue_2) ; X
    (for _index_2 (range 0 _returnvalue_2) ; Y
      (bind _returnvalue_5 (Class|FastNoiseWrapper|GetNoise2D _returnvalue_4 (* (+ _index (Math|Float|Floor _x)) 0.01) (* (+ _index_2 (Math|Float|Floor _y)) 0.01)))
      (Components|InstancedStaticMesh|AddInstance (Variables|Default|GetH_Cube) (Math|Transform|MakeTransform (Math|Vector|MakeVector (* _index 1e+02) (* _index_2 1e+02) (* (Math|Conversions|ToFloat(Integer) (Math|Float|Floor (* _returnvalue_5 2e+01))) 1e+02)) "0, 0, 0" "1,1,1")))))