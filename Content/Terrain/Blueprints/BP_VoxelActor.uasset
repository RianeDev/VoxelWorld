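; Voxel terrain actor that computes a 2D height map for one chunk; no mesh building is present and its event and construction graphs are empty.
; CalculateNoise offsets each cell by the chunk indices, sums weighted FastNoise samples at several scales, with the finest clamped non-negative, and floors the result into an integer height array.
; A new noise wrapper is constructed for every cell, and two layers sample identical coordinates.
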(event EventBeginPlay)

(event Collision|EventActorBeginOverlap
  (params (OtherActor :type Actor%20Object%20Reference)))

(event EventTick
  (params (DeltaSeconds :type Float%20%28single-precision%29)))

(fn ConstructionScript)

(fn CalculateNoise
  (bind _chunklineelements (Variables|Default|GetChunkLineElements))
  (bind _returnvalue (- _chunklineelements 1))
  (for _index (range 0 _returnvalue) ; Y
    (LocalVariables|SetLocalY _index)
    (for _index_2 (range 0 _returnvalue) ; X
      (LocalVariables|SetLocalX _index_2)
      (bind _returnvalue_2 (Game|ConstructObjectfromClass "/Script/FastNoiseGenerator.FastNoiseWrapper" self))
      (Class|FastNoiseWrapper|SetupFastNoise _returnvalue_2 "Simplex" 1337 (Variables|Default|GetFrequency) "Quintic" "FBM" 3 2.0 0.5 0.45 "Euclidean" "CellValue")
      (bind _returnvalue_3 (Class|FastNoiseWrapper|GetNoise2D _returnvalue_2 (* (+ (LocalVariables|GetLocalX) (* (Variables|Default|GetChunkXIndex) (Variables|Default|GetChunkLineElements))) 0.01) (* (+ (LocalVariables|GetLocalY) (* (Variables|Default|GetChunkYIndex) (Variables|Default|GetChunkLineElements))) 0.01)))
      (bind _returnvalue_4 (Class|FastNoiseWrapper|GetNoise2D _returnvalue_2 (* (+ (LocalVariables|GetLocalX) (* (Variables|Default|GetChunkXIndex) (Variables|Default|GetChunkLineElements))) 0.01) (* (+ (LocalVariables|GetLocalY) (* (Variables|Default|GetChunkYIndex) (Variables|Default|GetChunkLineElements))) 0.01)))
      (bind _returnvalue_5 (Class|FastNoiseWrapper|GetNoise2D _returnvalue_2 (* (+ (LocalVariables|GetLocalX) (* (Variables|Default|GetChunkXIndex) (Variables|Default|GetChunkLineElements))) 0.004) (* (+ (LocalVariables|GetLocalY) (* (Variables|Default|GetChunkYIndex) (Variables|Default|GetChunkLineElements))) 0.004)))
      (bind _returnvalue_6 (Class|FastNoiseWrapper|GetNoise2D _returnvalue_2 (* (+ (LocalVariables|GetLocalX) (* (Variables|Default|GetChunkXIndex) (Variables|Default|GetChunkLineElements))) 0.05) (* (+ (LocalVariables|GetLocalY) (* (Variables|Default|GetChunkYIndex) (Variables|Default|GetChunkLineElements))) 0.05)))
      (Utilities|Array|Add (LocalVariables|GetLocalNoise) (Math|Float|Floor (+ (* _returnvalue_3 4.0) (* _returnvalue_4 8.0) (* _returnvalue_5 16.0) (Math|Float|Clamp(Float) (* _returnvalue_6 4.0) 0.0 5.0))))))
  (return (LocalVariables|GetLocalNoise)))