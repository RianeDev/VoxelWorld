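; Voxel terrain chunk actor that builds a block landscape as a procedural mesh with collision from its construction script.
; SpawnChunk samples fixed-seed Perlin noise at world-space columns to fill a flat Size³ block array with ground and air.
; Only solid-block faces passing the neighbor Check are added to the mesh section.
; Neighbors beyond the sides or bottom count as open; those above the top do not.
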(event EventBeginPlay)

(event Collision|EventActorBeginOverlap
  (params (OtherActor :type Actor%20Object%20Reference)))

(event EventTick
  (params (DeltaSeconds :type Float%20%28single-precision%29)))

(fn ConstructionScript
  (CallFunction|SpawnChunk))

(fn CreateFace
  (params (Direction :type E_BlockDirection%20Enum :default "NewEnumerator0") (Scale :type Integer) (Position :type Int%20Vector%20Structure))
  (bind _vertexdata (Variables|Mesh|GetVertexData))
  (bind _returnvalue (Utilities|Array|Length _vertexdata))
  (bind _returnvalue_2 (- _returnvalue 4))
  (Utilities|Array|AppendArray (Variables|Mesh|GetVertexData) (CallFunction|GetFaceVertices Direction Scale Position))
  (Utilities|Array|AppendArray (Variables|Mesh|GetUVData) (Utilities|Array|MakeArray "(X=1.000000,Y=1.000000)" "(X=1.000000,Y=0.000000)" "" "(X=0.000000,Y=1.000000)"))
  (Utilities|Array|AppendArray (Variables|Mesh|GetTriangleData) (Utilities|Array|MakeArray (+ _returnvalue_2 3) (+ _returnvalue_2 2) _returnvalue_2 (+ _returnvalue_2 2) (+ _returnvalue_2 1) _returnvalue_2)))

(fn GetFaceVertices
  (params (Direction :type E_BlockDirection%20Enum :default "NewEnumerator0") (Scale :type Integer) (Position :type Int%20Vector%20Structure))
  (bind _data (LocalVariables|GetData))
  (for _index (range 0 3) ; Get each face vertice (4 total)
    (Utilities|Array|Add _data (+ (* (Utilities|Array|Get(acopy) (Variables|Constants|GetBlockVertexData) (Utilities|Array|Get(acopy) (Variables|Constants|GetBlockTriangleData) (+ _index (* (Math|Conversions|ToInteger(Byte) Direction) 4)))) Scale) (Math|Conversions|ToVector(Float) Position))))
  (return _data))

(fn IsEmpty
  (params (Block :type E_Block%20Enum :default "NewEnumerator0"))
  (return (or (Utilities|Enum|Equal(Enum) Block "NewEnumerator0") (Utilities|Enum|Equal(Enum) Block "NewEnumerator1"))))

(fn GetBlockIndex
  (params (Position :type Int%20Vector%20Structure))
  (bind _size (Variables|Constants|GetSize))
  ;[1 1 1] Get index between 0 and 4096 (chunk size)
  (return (+ (* (.x Position) _size) (.y Position) (* (.z Position) _size _size))) ; Moves from Y, to X, to Z to get block index
)

(fn GetPositionDirection
  (params (Direction :type E_BlockDirection%20Enum :default "NewEnumerator0") (Position :type Int%20Vector%20Structure))
  (switch Utilities|FlowControl|Switch|SwitchonE_BlockDirection Direction
    (:NewEnumerator0
      (return (Utilities|Struct|MakeIntVector (+ (.x Position) 1) (.y Position) (.z Position))))
    (:NewEnumerator1
      (return (Utilities|Struct|MakeIntVector (.x Position) (+ (.y Position) 1) (.z Position))))
    (:NewEnumerator2
      (return (Utilities|Struct|MakeIntVector (- (.x Position) 1) (.y Position) (.z Position))))
    (:NewEnumerator3
      (return (Utilities|Struct|MakeIntVector (.x Position) (- (.y Position) 1) (.z Position))))
    (:NewEnumerator4
      (return (Utilities|Struct|MakeIntVector (.x Position) (.y Position) (+ (.z Position) 1))))
    (:NewEnumerator5
      (return (Utilities|Struct|MakeIntVector (.x Position) (.y Position) (- (.z Position) 1))))))

(fn Check
  (params (Position :type Int%20Vector%20Structure))
  (bind _size (Variables|Constants|GetSize))
  (if (Math|Boolean|ORBoolean (>= (.x Position) _size) (>= (.y Position) _size) (<= (.x Position) -1) (<= (.y Position) -1) (<= (.z Position) -1))
    (return true)
    (elif (>= (.z Position) (Variables|Constants|GetSize))
      (return false)
      (else
        (return (CallFunction|IsEmpty (Utilities|Array|Get(acopy) (Variables|ChunkData|GetBlocks) (CallFunction|GetBlockIndex (Utilities|Struct|MakeIntVector (.x Position) (.y Position) (.z Position))))))))))

(fn SpawnChunk
  (bind _returnvalue (Transformation|GetActorLocation))
  (bind _blocks (Variables|ChunkData|GetBlocks))
  (bind _size (Variables|Constants|GetSize))
  (bind _size_2 (Variables|Constants|GetSize))
  (bind _size_3 (Variables|Constants|GetSize))
  (bind _returnvalue_2 (- _size 1))
  (bind _returnvalue_3 (- _size_3 1))
  (Utilities|FlowControl|Sequence
    (:then_0
      ;[1 1 1] Resize: 16x16x16 = 4096
      (Utilities|Array|Resize (Variables|ChunkData|GetBlocks) (* _size_2 _size_2 _size_2))
      ;[1 1 1] Create noise and generate height map
      (bind _returnvalue_4 (Game|ConstructObjectfromClass "/Script/FastNoiseGenerator.FastNoiseWrapper" self))
      (Class|FastNoiseWrapper|SetupFastNoise _returnvalue_4 "Perlin" 1340 0.01 "Quintic" "FBM" 3 2.0 0.5 0.45 "Euclidean" "CellValue")
      (for _index (range 0 _returnvalue_3)
        (for _index_2 (range 0 _returnvalue_3)
          (bind _returnvalue_5 (Class|FastNoiseWrapper|GetNoise2D _returnvalue_4 (* (+ (.x _returnvalue) (Math|Conversions|ToFloat(Integer) (* _index 100))) (Variables|Default|GetNoiseScaleX)) (* (+ (Math|Conversions|ToFloat(Integer) (* _index_2 100)) (.y _returnvalue)) (Variables|Default|GetNoiseScaleY)))) ; Value between -1 and 1
          ;;[1 1 1] Fills array with blocks
          (for _index_3 (range 0 (Math|Float|Truncate (* (Variables|Constants|GetSize) (/ (+ _returnvalue_5 1.0) 2.0)))) ; Ground blocks
            ;[1 1 1] Set Block types
            (Utilities|Array|SetArrayElem _blocks (CallFunction|GetBlockIndex (Utilities|Struct|MakeIntVector _index _index_2 _index_3)) "NewEnumerator2"))
          (for _index_4 (range (Math|Float|Truncate (* (Variables|Constants|GetSize) (/ (+ _returnvalue_5 1.0) 2.0))) (- (Variables|Constants|GetSize) 1)) ; Air blocks
            (Utilities|Array|SetArrayElem _blocks (CallFunction|GetBlockIndex (Utilities|Struct|MakeIntVector _index _index_2 _index_3)) "NewEnumerator1")))))
    (:then_1
      ;[1 1 1] Get X, Y, Z
      (for _index_5 (range 0 _returnvalue_2) ; X Value
        (LocalVariables|SetXValue _index_5)
        (for _index_6 (range 0 _returnvalue_2) ; Y Value
          (LocalVariables|SetYValue _index_6)
          (for _index_7 (range 0 _returnvalue_2) ; Z Value
            (LocalVariables|SetZValue _index_7)
            ;[1 1 1] Generate faces
            (if (not (CallFunction|IsEmpty (Utilities|Array|Get(acopy) (Variables|ChunkData|GetBlocks) (CallFunction|GetBlockIndex (Utilities|Struct|MakeIntVector (LocalVariables|GetXValue) (LocalVariables|GetYValue) (LocalVariables|GetZValue))))))
              (bind _enumvalue (|ForEachE_BlockDirection)
                (:LoopBody
                  (if (CallFunction|Check (CallFunction|GetPositionDirection _enumvalue (Utilities|Struct|MakeIntVector (LocalVariables|GetXValue) (LocalVariables|GetYValue) (LocalVariables|GetZValue))))
                    (CallFunction|CreateFace _enumvalue (Variables|Constants|GetScale) (Utilities|Struct|MakeIntVector (* (LocalVariables|GetXValue) 100) (* (LocalVariables|GetYValue) 100) (* (LocalVariables|GetZValue) 100)))))))))))
    (:then_2
      (Class|ProceduralMeshComponent|CreateMeshSectionLinearColor (Variables|Default|GetProceduralMesh) 0 (Variables|Mesh|GetVertexData) (Variables|Mesh|GetTriangleData) 0 (Variables|Mesh|GetUVData) 0 0 0 0 0 true))))